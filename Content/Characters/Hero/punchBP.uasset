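; Short-lived hero punch actor that plays a fight sound on BeginPlay and deals damage through a sphere.
; It destroys itself after a delay equal to the flipbook's framerate divided by 100.
; When the sphere begins an overlap, it prints a debug string and applies damage to all currently overlapping actors except player 0's character.
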(event OnComponentBeginOverlap(Sphere)
  (params (OverlappedComponent :type Primitive%20Component%20Object%20Reference) (OtherActor :type Actor%20Object%20Reference) (OtherComp :type Primitive%20Component%20Object%20Reference) (OtherBodyIndex :type Integer) (bFromSweep :type Boolean) (SweepResult :type Hit%20Result%20Structure%20%28by%20ref%29))
  (bind _sphere (Variables|Default|GetSphere))
  ;[0.6452 1 0.7621] Deal Damage
  (Development|PrintString "Degat")
  (for _array_element (Collision|GetOverlappingActors _sphere 0 :!class /Script/Engine.PrimitiveComponent)
    (if (!= _array_element _sphere)
      (if (!= _array_element (Game|GetPlayerCharacter 0))
        (Game|Damage|ApplyDamage _array_element (Variables|Default|GetDamage) 0 self)))))

(event EventBeginPlay
  ;[1 0.4463 0.4862] Sound
  (Utilities|FlowControl|Sequence
    (:then_0
      (Audio|PlaySound2D "/Game/Font/Musique/Héros/Fight_Sound.Fight_Sound" 1.0 1.0 0.4 0 0))
    (:then_1
      ;[1 0.9134 0.3997] Animation punch
      (Utilities|FlowControl|Delay (/ (Class|PaperFlipbookComponent|GetFlipbookFramerate (Variables|Default|Get%20flipBook)) 1e+02))
      (Actor|DestroyActor))))

(fn ConstructionScript)