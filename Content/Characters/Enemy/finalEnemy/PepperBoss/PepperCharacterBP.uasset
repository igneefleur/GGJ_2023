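; PepperCharacterBP is the Pepper boss enemy character, which chases the player and deals contact damage.
; PawnSensing sets a seeing flag, never cleared here, and triggers an AIMoveTo toward the player.
; Any DetectionBox overlap starts a one-second delay loop damaging the player until an end overlap clears the flag.
; A HItCheck function, uncalled here, applies damage without a set amount to overlapping Betterave actors; debug prints remain throughout.
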(event OnSeePawn(PawnSensing)
  (params (Pawn :type Pawn%20Object%20Reference))
  ;[0.3594 0.3594 0.3594] Chase the player
  (Development|PrintString "Je te vois")
  (Variables|Default|SetIs%20Seeing%20Player true)
  (CallFunction|FollowPlayer)
  (Development|PrintString (Utilities|String|ToString(Boolean) (Variables|Default|GetIs%20Seeing%20Player)) true true "(R=0.327744,G=0.139947,B=1.000000,A=1.000000)"))

(event OnComponentBeginOverlap(DetectionBox)
  (params (OverlappedComponent :type Primitive%20Component%20Object%20Reference) (OtherActor :type Actor%20Object%20Reference) (OtherComp :type Primitive%20Component%20Object%20Reference) (OtherBodyIndex :type Integer) (bFromSweep :type Boolean) (SweepResult :type Hit%20Result%20Structure%20%28by%20ref%29))
  (bind _basedamage (Variables|Default|GetBaseDamage))
  (bind _returnvalue (Math|Conversions|ToFloat(Integer) _basedamage))
  ;[1 0.08476 0.2651] Damage on body
  (Variables|Default|SetdealingDamage true)
  (Game|Damage|ApplyDamage (Game|GetPlayerCharacter 0) _returnvalue 0 self :!label _label)
  (Development|PrintString (Utilities|String|ToString(Float) _returnvalue) true true "(R=0.800000,G=0.000000,B=0.000000,A=1.000000)")
  (Utilities|FlowControl|Delay 1.0)
  (Development|PrintString "------------------")
  (Development|PrintString (Utilities|String|ToString(Boolean) (Variables|Default|GetdealingDamage)))
  (if (Variables|Default|GetdealingDamage)
    (goto _label)))

(event OnComponentEndOverlap(DetectionBox)
  (params (OverlappedComponent :type Primitive%20Component%20Object%20Reference) (OtherActor :type Actor%20Object%20Reference) (OtherComp :type Primitive%20Component%20Object%20Reference) (OtherBodyIndex :type Integer))
  ;[1 0.08476 0.2651] Damage on body
  (Variables|Default|SetdealingDamage false))

(event Custom|Follow%20Player
  ;[0.3594 0.3594 0.3594] Chase the player
  (if (Variables|Default|GetIs%20Seeing%20Player)
    (AI|AIMoveTo self "0, 0, 0" (Game|GetPlayerCharacter 0) 5.0 false
      (:OnSuccess
        (Development|PrintString "Je bouge !" true true "(R=1.000000,G=0.416946,B=0.889428,A=1.000000)"))
      (:OnFail
        (Development|PrintString "Immobile" true true "(R=0.140549,G=0.328125,B=0.136902,A=1.000000)")))))

(fn ConstructionScript)

(fn HItCheck
  (for _array_element (Collision|GetOverlappingActors (Variables|Default|GetDetectionBox) "/Game/Characters/Tests/Betterave.Betterave_C" :!class /Script/Engine.PrimitiveComponent)
    (if (!= _array_element self)
      (Game|Damage|ApplyDamage _array_element 0.0 0 0))))