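; Carrot enemy character with flipbook animation that chases the player and deals contact damage.
; Pawn sensing triggers an AI move toward the player, while DetectionBox damages actors that begin overlapping it.
; Incoming damage plays a hit flipbook that returns to walking when finished.
; Death stops movement and collision, then increments the kill counter on the parent EnemiesRoom actor.
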(event OnSeePawn(PawnSensing)
  (params (Pawn :type Pawn%20Object%20Reference))
  ;[0.3594 0.3594 0.3594] Chase the player
  (if (Variables|Default|GetisDead)
    (Components|DestroyComponent (Variables|Default|GetPawnSensing))
    (Sprite|SetFlipbook (Variables|Default|GetSprite) "/Game/Assets/Mobs/Carott/carottDeath_Flipbook.carottDeath_Flipbook")
    (else
      (Variables|Default|SetIs%20Seeing%20Player true)
      (CallFunction|FollowPlayer))))

(event OnComponentBeginOverlap(DetectionBox)
  (params (OverlappedComponent :type Primitive%20Component%20Object%20Reference) (OtherActor :type Actor%20Object%20Reference) (OtherComp :type Primitive%20Component%20Object%20Reference) (OtherBodyIndex :type Integer) (bFromSweep :type Boolean) (SweepResult :type Hit%20Result%20Structure%20%28by%20ref%29))
  ;[1 0 0] Do damage
  (Game|Damage|ApplyDamage OtherActor (Variables|Default|GetDamage) 0 0)
  (Development|PrintString "DamageDealt"))

(event OnFinishedPlaying(Sprite)
  (bind _sprite (Variables|Default|GetSprite))
  ;[1 1 1] Gestion Sprite animation carotte
  (if (not (Variables|Default|GetisDead))
    (Sprite|SetFlipbook _sprite "/Game/Assets/Mobs/Carott/carott_walk.carott_walk")
    (Components|Timeline|SetLooping _sprite true)
    (if (not (Audio|Components|Audio|IsPlaying _sprite))
      (Audio|Components|Audio|Play (Variables|Default|GetSprite)))))

(event Custom|Follow%20Player
  ;[0.3594 0.3594 0.3594] Chase the player
  (if (Variables|Default|GetIs%20Seeing%20Player)
    (AI|AIMoveTo self "0, 0, 0" (Game|GetPlayerCharacter 0) 5.0 false)))

(event Game|Damage|EventAnyDamage
  (params (Damage :type Float%20%28single-precision%29) (DamageType :type Damage%20Type%20Object%20Reference) (InstigatedBy :type Controller%20Object%20Reference) (DamageCauser :type Actor%20Object%20Reference))
  ;[1 1 1] Receive Damage
  (bind _output_get (Variables|Default|SetLife (- (Variables|Default|GetLife) Damage)))
  (if (<= _output_get 0.0)
    ;;[0.1198 0.1198 0.1198] Death
    (Sprite|SetFlipbook (Variables|Default|GetSprite) "/Game/Assets/Mobs/Carott/carottDeath_Flipbook.carottDeath_Flipbook")
    (Variables|Default|SetisDead true)
    (Components|Timeline|SetLooping (Variables|Default|GetSprite) false)
    (Pawn|Components|CharacterMovement|DisableMovement (Variables|Character|GetCharacterMovement))
    (Collision|SetCollisionEnabled (Variables|Collision|GetCapsuleComponent) "NoCollision")
    (Components|DestroyComponent (Variables|Default|GetDetectionBox))
    ;[1 1 1] notify Enemies Room
    (bind _asenemies_room (Utilities|Casting|CastToEnemiesRoom (Actor|GetParentActor self)))
    (Default|IncrementKillCounter _asenemies_room)
    (else
      (Sprite|SetFlipbook (Variables|Default|GetSprite) "/Game/Assets/Mobs/Carott/CarottTakeDamagedam.CarottTakeDamagedam")
      (Components|Timeline|SetLooping (Variables|Default|GetSprite) false))))

(fn ConstructionScript)

(fn HItCheck
  (for _array_element (Collision|GetOverlappingActors (Variables|Default|GetDetectionBox) "/Game/Characters/Tests/Betterave.Betterave_C" :!class /Script/Engine.PrimitiveComponent)
    (if (!= _array_element self)
      (Game|Damage|ApplyDamage _array_element 0.0 0 0))))