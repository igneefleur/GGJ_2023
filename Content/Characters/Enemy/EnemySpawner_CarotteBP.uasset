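; Enemy spawner that creates waves of Carotte enemies at its own location.
; On BeginPlay it casts the player character to Betterave and binds SpawnEnemy to that character's respawn-next-wave event.
; Each wave loop-spawns Carotte_Blueprint actors, ignoring collisions, based on EnemySpawned.
; It then raises SpawnIncrement and adds it to EnemySpawned, so waves grow by a larger step each time.
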(event Custom|SpawnEnemy
  ;[1 1 1] Spawn system
  (for _array_element (Utilities|Array|MakeArray 0 (- (Variables|Default|GetEnemySpawned) 0))
    (Game|SpawnActorfromClass "/Game/Characters/Enemy/Carotte_test/Carotte_Blueprint.Carotte_Blueprint_C" (Transformation|GetActorTransform) "AlwaysSpawn" 0 0))
  (Math|Integer|IncrementInt (Variables|Default|GetSpawnIncrement)
    (:%20%20
      (Variables|Default|SetEnemySpawned (+ (Variables|Default|GetEnemySpawned) (Variables|Default|GetSpawnIncrement))))))

(event EventBeginPlay
  (bind _asbetterave (Utilities|Casting|CastToBetterave (Game|GetPlayerCharacter 0)))
  (EventDispatchers|BindEventtoRespawnNextWave _asbetterave (delegate Custom|SpawnEnemy)))

(fn ConstructionScript)