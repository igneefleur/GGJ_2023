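; DamageBP is a damage volume that repeatedly hurts the player while its Box is overlapped.
; Any begin overlap sets DealingDamage and starts a one-second Delay loop applying random damage to player character 0, regardless of which actor entered.
; End overlap clears the flag, which the loop checks after each delay.
; Debug prints show the flag and a random value rolled separately from the damage dealt.
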(event OnComponentBeginOverlap(Box)
  (params (OverlappedComponent :type Primitive%20Component%20Object%20Reference) (OtherActor :type Actor%20Object%20Reference) (OtherComp :type Primitive%20Component%20Object%20Reference) (OtherBodyIndex :type Integer) (bFromSweep :type Boolean) (SweepResult :type Hit%20Result%20Structure%20%28by%20ref%29))
  (bind _returnvalue (Math|Random|RandomFloatinRange 5.0 2e+01))
  (Variables|Default|SetdealingDamage true)
  (Game|Damage|ApplyDamage (Game|GetPlayerCharacter 0) _returnvalue 0 self :!label _label)
  (Development|PrintString (Utilities|String|ToString(Float) _returnvalue) true true "(R=0.800000,G=0.000000,B=0.000000,A=1.000000)")
  (Utilities|FlowControl|Delay 1.0)
  (Development|PrintString "------------------")
  (Development|PrintString (Utilities|String|ToString(Boolean) (Variables|Default|GetdealingDamage)))
  (if (Variables|Default|GetdealingDamage)
    (goto _label)))

(event OnComponentEndOverlap(Box)
  (params (OverlappedComponent :type Primitive%20Component%20Object%20Reference) (OtherActor :type Actor%20Object%20Reference) (OtherComp :type Primitive%20Component%20Object%20Reference) (OtherBodyIndex :type Integer))
  (Variables|Default|SetdealingDamage false))

(fn ConstructionScript)